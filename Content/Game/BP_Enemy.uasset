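; BP_Enemy is an enemy actor that takes projectile hits and drops a weapon on death.
; On BeginPlay it caches the player character, clears its boss flag and scales its health to the player's level.
; Projectile hits destroy the projectile and subtract the player's equipped item damage.
; On death it spawns a BP_Weapon in its place, awards experience and triggers the player's experience check.
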(event EventBeginPlay
  (Variables|Default|SetisBoss false)
  (bind _asbp_first_person_character (Utilities|Casting|CastToBP_FirstPersonCharacter (Game|GetPlayerCharacter 0)))
  (Variables|Default|SetFirstPersonCharacter _asbp_first_person_character)
  (CallFunction|SetUpEnemy))

(event Collision|EventHit
  (params (MyComp :type Primitive%20Component%20Object%20Reference) (Other :type Actor%20Object%20Reference) (OtherComp :type Primitive%20Component%20Object%20Reference) (bSelfMoved :type Boolean) (HitLocation :type Vector :default "0, 0, 0") (HitNormal :type Vector :default "0, 0, 0") (NormalImpulse :type Vector :default "0, 0, 0") (Hit :type Hit%20Result%20Structure%20%28by%20ref%29))
  (Utilities|Casting|CastToBP_FirstPersonProjectile Other)
  (Actor|DestroyActor Other)
  (CallFunction|CheckEnemyHealth))

(fn ConstructionScript)

(fn CheckEnemyHealth
  (params (Weapon :type BP%20Weapon%20Object%20Reference))
  (bind _returnvalue (Transformation|GetActorTransform))
  (bind _firstpersoncharacter (Variables|Default|GetFirstPersonCharacter))
  (Variables|/Game/FirstPerson/Blueprints/BP_FirstPersonCharacter.BP_FirstPersonCharacter_C|SetbossKilled (Variables|Default|GetFirstPersonCharacter) (Variables|Default|GetisBoss))
  (Variables|Default|Sethealth (- (Variables|Default|Gethealth) (.damage (Variables|/Game/Game/BPC_Inventory.BPC_Inventory_C|GetEquippedItem (Variables|/Game/FirstPerson/Blueprints/BP_FirstPersonCharacter.BP_FirstPersonCharacter_C|GetBPC_Inventory (Variables|Default|GetFirstPersonCharacter))))))
  (if (<= (Variables|Default|Gethealth) 0)
    (Actor|DestroyActor)
    (bind _returnvalue_2 (Game|SpawnActorfromClass "/Game/Game/BP_Weapon.BP_Weapon_C" _returnvalue "Undefined" 0 0))
    (Variables|/Game/Game/BP_Weapon.BP_Weapon_C|SetPositionTransform _returnvalue_2 _returnvalue)
    (Variables|/Game/FirstPerson/Blueprints/BP_FirstPersonCharacter.BP_FirstPersonCharacter_C|SetexperiencePoints _firstpersoncharacter (+ (Variables|/Game/FirstPerson/Blueprints/BP_FirstPersonCharacter.BP_FirstPersonCharacter_C|GetexperiencePoints _firstpersoncharacter) (Variables|Default|GetexperiencePointsToAdd)))
    (Default|CheckExperience _firstpersoncharacter)))

(fn SetUpEnemy
  (Variables|Default|SetexperiencePointsToAdd 25)
  (if (== (Variables|/Game/FirstPerson/Blueprints/BP_FirstPersonCharacter.BP_FirstPersonCharacter_C|GetLevel (Variables|Default|GetFirstPersonCharacter)) 0)
    (Variables|Default|Sethealth 3)
    (elif (== (Variables|/Game/FirstPerson/Blueprints/BP_FirstPersonCharacter.BP_FirstPersonCharacter_C|GetLevel (Variables|Default|GetFirstPersonCharacter)) 1)
      (Variables|Default|Sethealth 15)
      (elif (== (Variables|/Game/FirstPerson/Blueprints/BP_FirstPersonCharacter.BP_FirstPersonCharacter_C|GetLevel (Variables|Default|GetFirstPersonCharacter)) 2)
        (Variables|Default|Sethealth 20)
        (elif (== (Variables|/Game/FirstPerson/Blueprints/BP_FirstPersonCharacter.BP_FirstPersonCharacter_C|GetLevel (Variables|Default|GetFirstPersonCharacter)) 3)
          (Variables|Default|Sethealth 30))))))