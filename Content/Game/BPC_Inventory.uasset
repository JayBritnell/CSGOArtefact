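; BPC_Inventory is an inventory component that holds a weapon array, the equipped item and a coin balance.
; Adding or dropping a weapon keeps CurrentIndex in step with the array.
; Dropping skips "null"-type slots and converts the removed weapon into coins, paying more for Legendary ones.
; Equipping swaps the chosen slot with the equipped item through a buffer, while separate functions add and subtract coins without bounds checks.
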(fn AddItem
  (params (NewItem :type Struct%20Weapon%20Structure%20%28by%20ref%29))
  (Utilities|Array|Add (Variables|Default|GetWeapons) NewItem)
  (Math|Integer|IncrementInt (Variables|Default|GetcurrentIndex)))

(fn DropItem
  (params (index :type Integer))
  (bind _weapons (Variables|Default|GetWeapons))
  (if (Utilities|Enum|NotEqual(Enum) (.type (Utilities|Array|Get(acopy) _weapons index)) "null")
    (if (Utilities|Enum|Equal(Enum) (.type (Utilities|Array|Get(acopy) _weapons index)) "Legendary")
      (Variables|Default|SetcoinsToAdd 50)
      (else
        (Variables|Default|SetcoinsToAdd 25)))
    (CallFunction|AddCoins (Variables|Default|GetcoinsToAdd))
    (Utilities|Array|RemoveIndex _weapons index)
    (Math|Integer|DecrementInt (Variables|Default|GetcurrentIndex))))

(fn EquipItem
  (params (index :type Integer))
  (bind _weapons (Variables|Default|GetWeapons))
  (bind _output_get (Variables|Default|SetbufferWeapon (Variables|Default|GetEquippedItem)))
  (Variables|Default|SetEquippedItem (Utilities|Array|Get(acopy) _weapons index))
  (Utilities|Array|SetArrayElem _weapons index _output_get))

(fn AddCoins
  (params (CoinsToAdd :type Integer))
  (Variables|Default|SetCoins (+ CoinsToAdd (Variables|Default|GetCoins))))

(fn RemoveCoins
  (params (CoinsToRemove :type Integer))
  (Variables|Default|SetCoins (- (Variables|Default|GetCoins) CoinsToRemove)))