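; BP_Chest is a chest actor that stores weapons and trades them with the first-person player's inventory.
; On BeginPlay it registers itself on the player character, and overlap events toggle CanOpenChest, which stays set on exit while the chest screen is open.
; Functions add items, move non-null items into the player's inventory component if room remains, and bubble-sort weapons by ascending damage.
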(event EventBeginPlay
  (bind _asbp_first_person_character (Utilities|Casting|CastToBP_FirstPersonCharacter (Game|GetPlayerCharacter 0)))
  (Variables|Default|SetBP%20First%20Person%20Character _asbp_first_person_character)
  (Variables|/Game/FirstPerson/Blueprints/BP_FirstPersonCharacter.BP_FirstPersonCharacter_C|SetBP_Chest _asbp_first_person_character self))

(event Collision|EventActorBeginOverlap
  (params (OtherActor :type Actor%20Object%20Reference))
  (bind _asbp_first_person_character (Utilities|Casting|CastToBP_FirstPersonCharacter OtherActor))
  (Variables|/Game/FirstPerson/Blueprints/BP_FirstPersonCharacter.BP_FirstPersonCharacter_C|SetCanOpenChest _asbp_first_person_character true))

(event Collision|EventActorEndOverlap
  (params (OtherActor :type Actor%20Object%20Reference))
  (bind _asbp_first_person_character (Utilities|Casting|CastToBP_FirstPersonCharacter OtherActor))
  (if (not (Variables|/Game/FirstPerson/Blueprints/BP_FirstPersonCharacter.BP_FirstPersonCharacter_C|GetChestScreenOpen (Variables|Default|GetBP%20First%20Person%20Character)))
    (Variables|/Game/FirstPerson/Blueprints/BP_FirstPersonCharacter.BP_FirstPersonCharacter_C|SetCanOpenChest _asbp_first_person_character false)))

(fn ConstructionScript)

(fn ChestAddItem
  (params (NewItem :type Struct%20Weapon%20Structure))
  (Utilities|Array|Add (Variables|Default|GetWeapons) NewItem)
  (Math|Integer|IncrementInt (Variables|Default|GetcurrentIndex)))

(fn ChestRemoveItem
  (params (index :type Integer))
  (bind _weapons (Variables|Default|GetWeapons))
  (bind _bp_first_person_character (Variables|Default|GetBP%20First%20Person%20Character))
  (bind _bpc_inventory (Variables|/Game/FirstPerson/Blueprints/BP_FirstPersonCharacter.BP_FirstPersonCharacter_C|GetBPC_Inventory _bp_first_person_character))
  (if (Utilities|Enum|NotEqual(Enum) (.type (Utilities|Array|Get(acopy) (Variables|Default|GetWeapons) index)) "null")
    (if (<= (Variables|/Game/Game/BPC_Inventory.BPC_Inventory_C|GetcurrentIndex _bpc_inventory) 9)
      (Default|AddItem _bpc_inventory (Utilities|Array|Get(acopy) _weapons index))
      (Utilities|Array|RemoveIndex _weapons index)
      (Math|Integer|DecrementInt (Variables|Default|GetcurrentIndex)))))

(fn SortChestItems
  (bind _currentindex (Variables|Default|GetcurrentIndex))
  (bind _weapons (Variables|Default|GetWeapons))
  (bind _weapons_2 (Variables|Default|GetWeapons))
  (for _index (range 0 (- _currentindex 1))
    (for _index_2 (range 0 (- _currentindex 2))
      (if (> (.damage (Utilities|Array|Get(acopy) _weapons_2 _index_2)) (.damage (Utilities|Array|Get(acopy) _weapons_2 (+ _index_2 1))))
        (Variables|Default|SetbufferWeapon (Utilities|Array|Get(acopy) (Variables|Default|GetWeapons) (+ _index_2 1)))
        (Utilities|Array|SetArrayElem _weapons (+ _index_2 1) (Utilities|Array|Get(acopy) (Variables|Default|GetWeapons) _index_2))
        (Utilities|Array|SetArrayElem _weapons _index_2 (Variables|Default|GetbufferWeapon))))))