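; BPC_Bounties is a component that holds a two-slot list of bounty objects for the game.
; On BeginPlay it constructs a single BPO_Bounty and places that same instance in both slots of the Bounties array.
; SetBounties calls Init on each entry, so the shared object initialises twice, and GetBountyInformation returns the BountyDescription at a given index.
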(event EventBeginPlay
  (bind _returnvalue (Game|ConstructObjectfromClass "/Game/Game/BPO_Bounty.BPO_Bounty_C"))
  (Variables|Default|SetBounties (Utilities|Array|MakeArray _returnvalue _returnvalue)))

(fn SetBounties
  (bind _bounties (Variables|Default|GetBounties))
  (Development|PrintString "initialise values")
  (for _index (range 0 1)
    (Default|Init (Utilities|Array|Get(acopy) _bounties _index))
    (Utilities|Array|SetArrayElem _bounties _index (Utilities|Array|Get(acopy) _bounties _index))))

(fn GetBountyInformation
  (params (index :type Integer))
  (return (Variables|/Game/Game/BPO_Bounty.BPO_Bounty_C|GetBountyDescription (Utilities|Array|Get(acopy) (Variables|Default|GetBounties) index))))