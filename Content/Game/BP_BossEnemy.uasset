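; Boss enemy Blueprint that takes hits from the first-person projectile.
; On BeginPlay it caches the player character, then flags itself as a boss and sets its starting Health, provided the cast succeeds.
; A projectile hit destroys the projectile and calls CheckEnemyHealth, which is not defined in this graph.
; The construction script only calls its parent.
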(event Collision|EventHit
  (params (MyComp :type Primitive%20Component%20Object%20Reference) (Other :type Actor%20Object%20Reference) (OtherComp :type Primitive%20Component%20Object%20Reference) (bSelfMoved :type Boolean) (HitLocation :type Vector :default "0, 0, 0") (HitNormal :type Vector :default "0, 0, 0") (NormalImpulse :type Vector :default "0, 0, 0") (Hit :type Hit%20Result%20Structure%20%28by%20ref%29))
  (Utilities|Casting|CastToBP_FirstPersonProjectile Other)
  (Actor|DestroyActor Other)
  (CallFunction|CheckEnemyHealth))

(event EventBeginPlay
  (bind _asbp_first_person_character (Utilities|Casting|CastToBP_FirstPersonCharacter (Game|GetPlayerCharacter 0)))
  (Variables|Default|SetFirstPersonCharacter _asbp_first_person_character)
  (Variables|Default|SetisBoss true)
  (Variables|Default|Sethealth 150))

(fn ConstructionScript
  (|CallParentFunction))