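; BP_Weapon is a randomized loot pickup that bobs and spins via a timeline after a random delay.
; On BeginPlay it rolls weighted rarity (always Legendary if the player's BossKilled is set), a level up to the player's, and a name.
; Rarity and level select a damage range, defined only for levels 1–3, for the final random damage.
; Player overlap adds it to the inventory and destroys it, or shows an inventory-full HUD notice.
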(event EventBeginPlay
  (bind _skeletalmesh (Variables|Default|GetSkeletalMesh))
  (bind _positiontransform (Variables|Default|GetPositionTransform))
  ;[1 1 1] Begin Play: When Weapon Spawned
  (bind _asbp_first_person_character (Utilities|Casting|CastToBP_FirstPersonCharacter (Game|GetPlayerCharacter 0)))
  (Variables|/Game/FirstPerson/Blueprints/BP_FirstPersonCharacter.BP_FirstPersonCharacter_C|SetBP_Weapon _asbp_first_person_character 0)
  (bind _output_get (Variables|Default|SetFirst%20Person%20Character _asbp_first_person_character))
  (CallFunction|SetUpWeaponStats (Variables|/Game/FirstPerson/Blueprints/BP_FirstPersonCharacter.BP_FirstPersonCharacter_C|GetbossKilled _output_get))
  (Utilities|FlowControl|Delay (Math|Random|RandomFloat))
  ;;[1 1 1] Simple Weapon Animation
  (bind (_direction _up_down _rotate) (Timeline|Timeline Play)
    (:Update
      (Transformation|SetRelativeLocation _skeletalmesh (Math|Vector|MakeVector (.x (.location _positiontransform)) (.y (.location _positiontransform)) (+ (.z (.location _positiontransform)) _up_down)) false false)
      (Transformation|SetRelativeRotation _skeletalmesh (Math|Rotator|MakeRotator 0.0 0.0 _rotate) false false))))

(event Collision|EventActorBeginOverlap
  (params (OtherActor :type Actor%20Object%20Reference))
  ;[1 1 1] Picked up by Player
  (bind _asbp_first_person_character (Utilities|Casting|CastToBP_FirstPersonCharacter OtherActor))
  (if (< (Variables|/Game/Game/BPC_Inventory.BPC_Inventory_C|GetcurrentIndex (Variables|/Game/FirstPerson/Blueprints/BP_FirstPersonCharacter.BP_FirstPersonCharacter_C|GetBPC_Inventory _asbp_first_person_character)) (Variables|/Game/Game/BPC_Inventory.BPC_Inventory_C|Getsize (Variables|/Game/FirstPerson/Blueprints/BP_FirstPersonCharacter.BP_FirstPersonCharacter_C|GetBPC_Inventory _asbp_first_person_character)))
    (Default|AddItem (Variables|/Game/FirstPerson/Blueprints/BP_FirstPersonCharacter.BP_FirstPersonCharacter_C|GetBPC_Inventory _asbp_first_person_character) (Utilities|Struct|MakeStruct_Weapon (Variables|Default|Getlevel) (Variables|Default|GetType) (Variables|Default|GetName) (Variables|Default|GetDamage)))
    (Actor|DestroyActor)
    (else
      (bind _asbp_first_person_character_2 (Utilities|Casting|CastToBP_FirstPersonCharacter (Game|GetPlayerCharacter 0)))
      (Default|InventoryFull (Variables|/Game/FirstPerson/Blueprints/BP_FirstPersonCharacter.BP_FirstPersonCharacter_C|GetW_HUD _asbp_first_person_character_2)))))

(fn ConstructionScript)

(fn SetUpWeaponStats
  (params (boss :type Boolean))
  (if boss
    (Variables|Default|SetType "Legendary")
    (bind _asbp_first_person_character (Utilities|Casting|CastToBP_FirstPersonCharacter (Game|GetPlayerCharacter 0) :!label _label))
    (if (> (Variables|/Game/FirstPerson/Blueprints/BP_FirstPersonCharacter.BP_FirstPersonCharacter_C|GetLevel _asbp_first_person_character) 0)
      (Variables|Default|Setlevel (Math|Random|RandomIntegerinRange 1 (Variables|/Game/FirstPerson/Blueprints/BP_FirstPersonCharacter.BP_FirstPersonCharacter_C|GetLevel _asbp_first_person_character)))
      (else
        (Variables|Default|Setlevel 1)))
    (Utilities|FlowControl|Sequence
      (:then_0
        (if (Utilities|Enum|Equal(Enum) (Variables|Default|GetType) "Legendary")
          (Variables|Default|SetName (.OutItem (Utilities|Array|Random (Variables|Default|GetLegendaryNames))))
          (else
            (Variables|Default|SetName (.OutItem (Utilities|Array|Random (Variables|Default|GetNames)))))))
      (:then_1
        (CallFunction|CheckWeapon)))
    (else
      (Variables|Default|SetRandomNumber (Math|Random|RandomIntegerinRange 1 25))
      (if (== (Variables|Default|GetRandomNumber) 25)
        (Variables|Default|SetType "Legendary")
        (goto _label)
        (elif (and (<= (Variables|Default|GetRandomNumber) 24) (>= (Variables|Default|GetRandomNumber) 22))
          (Variables|Default|SetType "Ultra Rare")
          (goto _label)
          (elif (and (<= (Variables|Default|GetRandomNumber) 21) (>= (Variables|Default|GetRandomNumber) 18))
            (Variables|Default|SetType "Rare")
            (goto _label)
            (elif (and (<= (Variables|Default|GetRandomNumber) 17) (>= (Variables|Default|GetRandomNumber) 11))
              (Variables|Default|SetType "Uncommon")
              (goto _label)
              (elif (and (<= (Variables|Default|GetRandomNumber) 10) (>= (Variables|Default|GetRandomNumber) 1))
                (Variables|Default|SetType "Common")
                (goto _label)
                (else
                  (Development|PrintString "Type not set"))))))))))

(fn CheckWeapon
  (bind _level (Variables|Default|Getlevel))
  (switch string (Variables|Default|GetType)
    (:Legendary
      (switch int _level
        (:1
          (Variables|Default|SetminimumDmg 7)
          (Variables|Default|SetmaximumDmg 10))
        (:2
          (Variables|Default|SetminimumDmg 18)
          (Variables|Default|SetmaximumDmg 20))
        (:3
          (Variables|Default|SetminimumDmg 29)
          (Variables|Default|SetmaximumDmg 30))))
    (:Ultra%20Rare
      (switch int _level
        (:1
          (Variables|Default|SetminimumDmg 5)
          (Variables|Default|SetmaximumDmg 6))
        (:2
          (Variables|Default|SetminimumDmg 15)
          (Variables|Default|SetmaximumDmg 17))
        (:3
          (Variables|Default|SetminimumDmg 27)
          (Variables|Default|SetmaximumDmg 28))))
    (:Rare
      (switch int _level
        (:1
          (Variables|Default|SetminimumDmg 3)
          (Variables|Default|SetmaximumDmg 4))
        (:2
          (Variables|Default|SetminimumDmg 13)
          (Variables|Default|SetmaximumDmg 14))
        (:3
          (Variables|Default|SetminimumDmg 25)
          (Variables|Default|SetmaximumDmg 26))))
    (:Uncommon
      (switch int _level
        (:1
          (Variables|Default|SetminimumDmg 2)
          (Variables|Default|SetmaximumDmg 2))
        (:2
          (Variables|Default|SetminimumDmg 12)
          (Variables|Default|SetmaximumDmg 12))
        (:3
          (Variables|Default|SetminimumDmg 23)
          (Variables|Default|SetmaximumDmg 24))))
    (:Common
      (switch int _level
        (:1
          (Variables|Default|SetminimumDmg 1)
          (Variables|Default|SetmaximumDmg 1))
        (:2
          (Variables|Default|SetminimumDmg 11)
          (Variables|Default|SetmaximumDmg 11))
        (:3
          (Variables|Default|SetminimumDmg 21)
          (Variables|Default|SetmaximumDmg 22)))))
  (CallFunction|SetWeaponDamage (Variables|Default|GetminimumDmg) (Variables|Default|GetmaximumDmg)))

(fn SetWeaponDamage
  (params (minimumDamage :type Integer) (maximumDamage :type Integer))
  (Variables|Default|SetDamage (Math|Random|RandomIntegerinRange minimumDamage maximumDamage)))