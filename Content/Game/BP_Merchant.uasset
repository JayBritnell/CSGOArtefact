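; Merchant actor that sells randomly generated Legendary weapons and holds bounties through a BPCBounties component.
; Registers itself with the first-person character and allows opening the merchant on overlap, revoking it on exit unless the screen is open.
; Fills StoreItems with random names and one of two damage values, refreshing stock and bounties on a Delay-throttled Tick countdown that is set tickable while paused.
; Helper functions remove individual items or bounties.
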(event EventBeginPlay
  (bind _asbp_first_person_character (Utilities|Casting|CastToBP_FirstPersonCharacter (Game|GetPlayerCharacter 0)))
  (Variables|Default|SetBP%20First%20Person%20Character _asbp_first_person_character)
  (Variables|/Game/FirstPerson/Blueprints/BP_FirstPersonCharacter.BP_FirstPersonCharacter_C|SetBP_Merchant _asbp_first_person_character self)
  (Class|Actor|SetTickablewhenPaused true)
  (Variables|Default|SetCurrentTime (Variables|Default|GetResetTime))
  (CallFunction|SetUpShopItems))

(event Collision|EventActorBeginOverlap
  (params (OtherActor :type Actor%20Object%20Reference))
  (bind _asbp_first_person_character (Utilities|Casting|CastToBP_FirstPersonCharacter OtherActor))
  (Variables|/Game/FirstPerson/Blueprints/BP_FirstPersonCharacter.BP_FirstPersonCharacter_C|SetCanOpenMerchant _asbp_first_person_character true))

(event Collision|EventActorEndOverlap
  (params (OtherActor :type Actor%20Object%20Reference))
  (bind _asbp_first_person_character (Utilities|Casting|CastToBP_FirstPersonCharacter OtherActor))
  (if (not (Variables|/Game/FirstPerson/Blueprints/BP_FirstPersonCharacter.BP_FirstPersonCharacter_C|GetMerchantScreenOpen (Variables|Default|GetBP%20First%20Person%20Character)))
    (Variables|/Game/FirstPerson/Blueprints/BP_FirstPersonCharacter.BP_FirstPersonCharacter_C|SetCanOpenMerchant _asbp_first_person_character false)))

(event EventTick
  (params (DeltaSeconds :type Float%20%28single-precision%29))
  (Utilities|FlowControl|Sequence
    (:then_0
      (Utilities|FlowControl|Delay 1.0)
      (Variables|Default|SetCurrentTime (- (Variables|Default|GetCurrentTime) 1.0)))
    (:then_1
      (if (== (Variables|Default|GetCurrentTime) 0.0)
        (CallFunction|SetUpShopItems)
        (Variables|Default|SetCurrentTime (Variables|Default|GetResetTime))))))

(fn ConstructionScript)

(fn SetUpShopItems
  (for _index (range 0 (Variables|Default|GetSize))
    (Variables|Default|SetWeaponLevel 3)
    (Variables|Default|SetWeaponType "Legendary")
    (Variables|Default|SetWeaponName (.OutItem (Utilities|Array|Random (Variables|Default|GetLegendaryNames))))
    (Variables|Default|SetRandomNumber (Math|Random|RandomIntegerinRange 1 2))
    (if (== (Variables|Default|GetRandomNumber) 1)
      (Variables|Default|SetWeaponDamage 29)
      (Utilities|Array|SetArrayElem (Variables|Default|GetStoreItems) _index (Utilities|Struct|MakeStruct_Weapon (Variables|Default|GetWeaponLevel) (Variables|Default|GetWeaponType) (Variables|Default|GetWeaponName) (Variables|Default|GetWeaponDamage)) true :!label _label)
      (elif (== (Variables|Default|GetRandomNumber) 2)
        (Variables|Default|SetWeaponDamage 30)
        (goto _label))))
  (Variables|Default|SetCurrentIndex (Variables|Default|GetSize))
  (Default|SetBounties (Variables|Default|GetBPC_Bounties)))

(fn MerchantRemoveItem
  (params (index :type Integer))
  (Utilities|Array|RemoveIndex (Variables|Default|GetStoreItems) index)
  (Math|Integer|DecrementInt (Variables|Default|GetCurrentIndex)))

(fn MerchantRemoveBounty
  (params (index :type Integer))
  (Utilities|Array|RemoveIndex (Variables|/Game/Game/BPC_Bounties.BPC_Bounties_C|GetBounties (Variables|Default|GetBPC_Bounties)) index))